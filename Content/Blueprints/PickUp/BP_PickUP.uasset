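; BP_PickUP is a pickup actor that the player's BP_Indio_Character collects by walking into its trigger.
; On BeginPlay it caches the Indio controller and character.
; On overlap it asks the controller's InventoryCheck for space, then passes itself to PickUpItem and hides with collision off rather than being destroyed.
; When the check fails it prints an inventory-full message.
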(event OnComponentBeginOverlap(Trigger)
  (params (OverlappedComponent :type Primitive%20Component%20Object%20Reference) (OtherActor :type Actor%20Object%20Reference) (OtherComp :type Primitive%20Component%20Object%20Reference) (OtherBodyIndex :type Integer) (bFromSweep :type Boolean) (SweepResult :type Hit%20Result%20Structure%20%28by%20ref%29))
  ;[0 0 0 1 12] PickUp the Item if has Space
  (Utilities|Casting|CastToBP_Indio_Character OtherActor)
  (bind _hasspace_ (Default|InventoryCheck (Variables|Default|GetControllerReference)))
  (if _hasspace_
    (Default|PickUpItem (Variables|Default|GetControllerReference) self)
    (Rendering|SetActorHiddenInGame true)
    (Collision|SetActorEnableCollision false)
    (else
      (Development|PrintString "Inventory Full"))))

(event EventBeginPlay
  ;[0 0 0 1 12] Get References of Player
  (bind _asbp_indio_controller (Utilities|Casting|CastToBP_Indio_Controller (Game|GetPlayerController 0)))
  (Variables|Default|SetControllerReference _asbp_indio_controller)
  (bind _asbp_indio_character (Utilities|Casting|CastToBP_Indio_Character (Game|GetPlayerCharacter 0)))
  (Variables|Default|SetCharacterReference _asbp_indio_character))

(fn ConstructionScript)