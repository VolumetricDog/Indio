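; BP_Indio_Controller is the controller for the Indio character and holds the player's item inventory.
; It caches the character on BeginPlay, checks InventoryObjects for invalid entries as free space, and puts picked-up items in the first empty slot.
; Pickup also copies the item's image to the matching HUD inventory button through the character's HUD reference.
; Item use check, move and remove functions are unimplemented stubs.
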(event EventBeginPlay
  ;[0 0 0 1 12] Referencing Character
  (bind _asbp_indio_character (Utilities|Casting|CastToBP_Indio_Character (Game|GetPlayerCharacter 0)))
  (Variables|Default|SetCharacterReference _asbp_indio_character))

(fn ConstructionScript)

(fn InventoryCheck
  (for _array_element (Variables|Default|GetInventoryObjects)
    (if (not (Utilities|IsValid _array_element))
      (Variables|Default|SetSpacesAvailable (+ (Variables|Default|GetSpacesAvailable) 1))))
  (if (> (Variables|Default|GetSpacesAvailable) 0)
    (Variables|Default|SetHasInventorySpace? true)
    (else
      (Variables|Default|SetHasInventorySpace? false)))
  (return (Variables|Default|GetHasInventorySpace?)))

(fn UserItemCheck)

(fn FindEmptySlot
  (bind (_array_element _array_index) (Utilities|Array|ForEachLoopwithBreak (Variables|Default|GetInventoryObjects) :!label _label)
    (:LoopBody
      (if (not (Utilities|IsValid _array_element))
        (bind _output_get (Variables|Default|SetEmptySlot _array_index))
        (goto _label Break)))
    (:Completed
      (return _output_get))))

(fn MoveItem
  (params (From :type Integer) (To :type Integer))
  (return false))

(fn MoveImage
  (params (From :type Integer) (To :type Integer) (ItemImage :type Texture%202D%20Object%20Reference) (Swapping :type Boolean)))

(fn PickUpItem
  (params (ItemToPickUp :type Object%20Object%20Reference))
  (Utilities|Array|SetArrayElem (Variables|Default|GetInventoryObjects) (CallFunction|FindEmptySlot) ItemToPickUp)
  (bind _asbp_pick_up (Utilities|Casting|CastToBP_PickUP ItemToPickUp))
  (Variables|/Game/Blueprints/UI/WG_InventorySlot.WG_InventorySlot_C|SetInventoryImage (Utilities|Array|Get(acopy) (Variables|/Game/Blueprints/UI/WG_Inventory.WG_Inventory_C|GetInventoryButton (Variables|/Game/Blueprints/UI/WG_HUD.WG_HUD_C|GetWG_Inventory (Variables|/Game/Blueprints/BP_Indio_Character.BP_Indio_Character_C|GetHUDReference (Variables|Default|GetCharacterReference)))) (Variables|Default|GetEmptySlot)) (Variables|/Game/Blueprints/PickUp/BP_PickUP.BP_PickUP_C|GetPickUpImage _asbp_pick_up))
  (return))

(fn RemoveItem)